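; BP_ENEMY is an enemy character that detects the player and performs a melee shove attack.
; Pawn sensing flags a seen Player-tagged pawn in the AI controller's Blackboard, and nothing here clears that flag.
; AttackPlayer plays a montage, immediately sphere-traces a short distance forward from an attack point, and applies damage to any pawn hit.
; An Attacking flag blocks re-triggering until the montage completes.
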(event OnSeePawn(PawnSensing)
  (params (Pawn :type Pawn%20Object%20Reference))
  (if (Actor|ActorHasTag Pawn "Player")
    (AI|Components|Blackboard|SetValueasBool (AI|GetBlackboard (AI|GetAIController self)) (Utilities|Name|MakeLiteralName "seeingPlayer") true)))

(event Custom|AttackPlayer
  (bind _attacktracepoint (Variables|Default|GetAttackTracePoint))
  (bind _returnvalue (Transformation|GetWorldLocation _attacktracepoint))
  (if (not (Variables|Default|Getattacking))
    (Variables|Default|Setattacking true)
    (Animation|Montage|PlayMontage (Variables|Character|GetMesh) "/Game/Enemy/Paired_PushShove_Att1_Montage.Paired_PushShove_Att1_Montage"
      (:then
        (bind (_outhit _returnvalue_2) (Collision|SphereTraceForObjects _returnvalue (+ _returnvalue (* (Math|Vector|GetForwardVector (Transformation|GetWorldRotation _attacktracepoint)) 7e+01)) 25.0 (Utilities|Array|MakeArray "ObjectTypeQuery3") false 0 "None"))
        (if _returnvalue_2
          (Game|Damage|ApplyDamage (.HitActor (Collision|BreakHitResult _outhit)) 1e+01 0 0)))
      (:OnCompleted
        (Variables|Default|Setattacking false)))))

(fn ConstructionScript)