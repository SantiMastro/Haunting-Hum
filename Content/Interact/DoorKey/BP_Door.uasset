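; BP_Door is an interactable door actor that swings open and closed only once its key has been picked up.
; The PickUpKey event sets HasKey, which Interact checks.
; With the key, Interact plays a squeak and a FlipFlop alternately plays or reverses DoorTimeline, which lerps the mesh's relative yaw.
; Without it, the door stays put and the sound call has no sound asset set.
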(event EventInteract
  (if (Variables|Default|GetHas%20Key?)
    (Audio|PlaySoundatLocation "/Game/Audio/346211__inspectorj__door-squeak-normal-e.346211__inspectorj__door-squeak-normal-e" (Transformation|GetActorLocation) "0, 0, 0" 1.0 1.0 0.0 0 0 0 0)
    (Utilities|FlowControl|FlipFlop
      (:A
        (bind _door_track (Timeline|Door%20Timeline Play)
          (:Update
            (Transformation|SetRelativeRotation (Variables|Default|GetStaticMesh) (Math|Rotator|MakeRotator 0.0 0.0 (Math|Float|Lerp 0.0 1.1e+02 _door_track)) false false))))
      (:B
        (Timeline|Door%20Timeline Reverse)))
    (else
      (Audio|PlaySoundatLocation 0 (Transformation|GetActorLocation) "0, 0, 0" 1.0 1.0 0.0 0 0 0 0))))

(event EventPickUpKey
  (Variables|Default|SetHas%20Key? true))

(fn ConstructionScript)