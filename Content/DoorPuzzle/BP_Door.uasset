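; BP_Door is a puzzle door that rotates its static mesh open and closed.
; On BeginPlay it caches the mesh's world rotation as the default.
; OpenDoor plays a timeline whose DoorAnim track supplies a yaw offset, combined with that default to set the world rotation each update.
; CloseDoor reverses the same timeline to swing the door back.
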(event Custom|OpenDoor
  (bind _dooranim (Timeline|DoorTimeline Play)
    (:Update
      (Transformation|SetWorldRotation (Variables|Debug|GetStaticMeshComponent) (Math|Rotator|CombineRotators (Math|Rotator|MakeRotator 0.0 0.0 _dooranim) (Variables|Default|GetDefaultRotation)) false false))))

(event Custom|CloseDoor
  (bind _dooranim (Timeline|DoorTimeline Reverse)
    (:Update
      (Transformation|SetWorldRotation (Variables|Debug|GetStaticMeshComponent) (Math|Rotator|CombineRotators (Math|Rotator|MakeRotator 0.0 0.0 _dooranim) (Variables|Default|GetDefaultRotation)) false false))))

(event EventBeginPlay
  (Variables|Default|SetDefaultRotation (Transformation|GetWorldRotation (Variables|Debug|GetStaticMeshComponent))))

(fn ConstructionScript)